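; BP_AttachmentsSave is a save object that stores weapon attachment builds and skins for guns.
; It keeps two maps keyed by weapon name, GunBuilds and GunSkins, each with an add and a get function.
; The getters print a "not found" message when no entry exists for the requested weapon.
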(fn `AddGunBuild`
  (params (WeaponName :type "Name (by ref)") (GunBuild :type "/Game/FPS_Test/Code/Weapon/Attachments/F_GunBuild Structure (by ref)"))
  (`BlueprintMapLibrary.Map_Add` (`self.GunBuilds`) WeaponName GunBuild))

(fn `AddGunSkin`
  (params (`Weapon Name` :type "Name (by ref)") (Skin :type "/Game/LowPolyAnimatedModernGuns/Demo/Core/Skins/BP_LPAMG_Skin Object Reference (by ref)"))
  (`BlueprintMapLibrary.Map_Add` (`self.GunSkins`) `Weapon Name` Skin))

(fn `GetGunBuild`
  (params (WeaponName :type Name))
  (returns (Value :type "/Game/FPS_Test/Code/Weapon/Attachments/F_GunBuild Structure"))
  (bind (_value _returnvalue) (`BlueprintMapLibrary.Map_Find` (`self.GunBuilds`) WeaponName))
  (if _returnvalue
    (return _value)
    (else
      (`KismetSystemLibrary.PrintString` null "Build not found"))))

(fn `GetGunSkin`
  (params (`Gun Name` :type "Name (by ref)"))
  (returns (Value :type "/Game/LowPolyAnimatedModernGuns/Demo/Core/Skins/BP_LPAMG_Skin Object Reference"))
  (bind (_value _returnvalue) (`BlueprintMapLibrary.Map_Find` (`self.GunSkins`) `Gun Name`))
  (if _returnvalue
    (return _value)
    (else
      (`KismetSystemLibrary.PrintString` null "Skin not found")
      (return null))))