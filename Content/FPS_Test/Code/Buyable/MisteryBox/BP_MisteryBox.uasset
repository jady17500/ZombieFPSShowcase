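; Buyable mystery box actor that sells a random weapon to the interacting player.
; Interacting requests a purchase through the player controller and AC_Buyable; completion triggers the replicated open on the server.
; A timeline lifts lid and display weapon while a looping timer randomly swaps the display's child actor class from the Weapons map keys.
; Once spinning stops, only the confirmed buyer can take the mapped weapon, which closes the box.
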(event `OpenBox`
  (`SceneComponent.SetHiddenInGame` (`self.DisplayWeapon`) false true)
  (set `self.IsOpen` true)
  (set `self.Start Rotation` (`SceneComponent.K2_GetComponentRotation` (`self.OpenPivot`)))
  (set `self.StartWeaponLocation` (`SceneComponent.K2_GetComponentLocation` (`self.DisplayWeapon`)))
  (bind (_direction _opening) (`Timeline|BoxOpen` :!via `PlayFromStart` :!label _label)
    (:`Update`
      (`SceneComponent.K2_SetWorldRotation` (`self.OpenPivot`) (`KismetMathLibrary.RLerp` (`self.Start Rotation`) (`KismetMathLibrary.MakeRotator` (.roll (`self.Start Rotation`)) 100.0 (.yaw (`self.Start Rotation`))) _opening) false false)
      (`SceneComponent.K2_SetWorldLocation` (`self.DisplayWeapon`) (`KismetMathLibrary.VLerp` (`self.StartWeaponLocation`) (`KismetMathLibrary.MakeVector` (.x (`self.StartWeaponLocation`)) (.y (`self.StartWeaponLocation`)) (+ (.z (`self.StartWeaponLocation`)) 65.0)) _opening) false false))))

(event `CloseBox`
  (`SceneComponent.SetHiddenInGame` (`self.DisplayWeapon`) true true)
  (`KismetSystemLibrary.K2_ClearAndInvalidateTimerHandle` (`self.BoxOpenTimeHandle`))
  (set `self.IsOpen` false)
  (goto _label :!via `ReverseFromEnd`))

(event `self.Interact`
  (params (Interactor :type "Actor Object Reference"))
  (if (`self.IsOpen`)
    (if (`self.IsSpinning`)
      _
      (elif (== (`self.ConfirmedBuyer`) Interactor)
        (message `/Game/FPS_Test/Code/Player/BPI_Player.AddWeaponToInventory` Interactor (`BlueprintMapLibrary.Map_Find` (`self.Weapons`) (`ChildActorComponent.ChildActorClass` (`self.DisplayWeapon`))) false)
        (if (`KismetSystemLibrary.IsServer`)
          (`self.CloseBox_Rep`)
          (else
            (`self.CloseBox_Server`)))))
    (else
      (bind _asbp_player_controller (cast `/Game/FPS_Test/Code/Player/BP_PlayerController` (`Pawn.GetController` (cast `Pawn` Interactor :!pure true))))
      (set `self.Buyer` Interactor)
      (`/Game/FPS_Test/Code/Player/BP_PlayerController.ServerBuyEvent` _asbp_player_controller (`self.GetComponentByClass` Interactor "/Script/ZombieFPS.CurrencyComponent") (`self.AC_Buyable`)))))

(event `self.AC_Buyable.OnBuyComplete`
  (if (`KismetSystemLibrary.IsServer`)
    (`self.BoxOpen_Rep`)))

(event `StartTickingWeapons`
  (set `self.IsSpinning` true)
  (bind _returnvalue (`KismetSystemLibrary.K2_SetTimerDelegate` (delegate `TickWeapons`) (`self.WeapontTickLenght`) true))
  (set `self.WeaponTickTimer` _returnvalue))

(event `TickWeapons`
  (bind _keys (`BlueprintMapLibrary.Map_Keys` (`self.Weapons`)))
  (`ChildActorComponent.SetChildActorClass` (`self.DisplayWeapon`) (`KismetArrayLibrary.Array_Random` _keys)))

(event `StopTickWeapons`
  (`KismetSystemLibrary.K2_ClearAndInvalidateTimerHandle` (`self.WeaponTickTimer`))
  (set `self.IsSpinning` false))

(event `OpenBox_Server`
  (`self.BoxOpen_Rep`))

(event `BoxOpen_Rep`
  (set `self.ConfirmedBuyer` (`self.Buyer`))
  (`self.OpenBox`)
  (`self.StartTickingWeapons`)
  (`KismetSystemLibrary.K2_SetTimerDelegate` (`|CreateDelegate` :!event `StopTickWeapons`) (`self.BoxSelectCoolDown`))
  (bind _returnvalue (`KismetSystemLibrary.K2_SetTimerDelegate` (`|CreateDelegate` :!event `CloseBox`) (`self.BoxOpenTime`)))
  (set `self.BoxOpenTimeHandle` _returnvalue))

(event `CloseBox_Rep`
  (`self.CloseBox`)
  (set `self.ConfirmedBuyer` null)
  (set `self.Buyer` null))

(event `CloseBox_Server`
  (`self.CloseBox_Rep`))

(fn `GetInteractText`
  (returns (OutText :type Text) (OutDescription :type Text) (ReturnValue :type Boolean))
  (bind _ac_buyable (`self.AC_Buyable`))
  (return (select `bool` (and (`self.IsOpen`) (not (`self.IsSpinning`))) :`false` (`|FormatText` "open the mistery box for {PRICE} {CURRENCY}" (`BuyableComponent.Price` _ac_buyable) (`BuyableComponent.RequiredCurrencyName` _ac_buyable)) :`true` "pick up weapon") "" true))

(fn `UserConstructionScript`)