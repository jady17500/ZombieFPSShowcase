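; Juggernog perk component that raises its owner's maximum health while the perk is held.
; On perk start, it adds a flat MaxHealth bonus through the owner's StatManagerComponent and adds its icon to the first player's perk container UI.
; On removal, it resets MaxHealth to the base stat value if one is found, and leaves the icon untouched.
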(event `self.PerkStartEvent`
  (`StatManagerComponent.IncreaseStatFlat` (`Actor.GetComponentByClass` (`self.GetOwner`) "/Script/ZombieFPS.StatManagerComponent") "MaxHealth" 150.0 false)
  (bind _widget (message `/Game/FPS_Test/Code/Player/BPI_Player.GetPlayerUi` (`GameplayStatics.GetPlayerCharacter` 0)))
  (`/Game/FPS_Test/Code/UI/Components/WBP_PerkContainer.Add Perk Icon` (`/Game/FPS_Test/Code/UI/Pages/WBP_MainUI.WBP_PerkContainer` _widget) (`self.PerkIconBrush`)))

(event `self.PerkRemoveEvent`
  (bind _returnvalue (`Actor.GetComponentByClass` (`self.GetOwner`) "/Script/ZombieFPS.StatManagerComponent"))
  (bind (_outstat _returnvalue_2) (`StatManagerComponent.GetBaseStat` _returnvalue "MaxHealth"))
  (if _returnvalue_2
    (`StatManagerComponent.ResetStatToPreviousValue` _returnvalue "MaxHealth" _outstat)))