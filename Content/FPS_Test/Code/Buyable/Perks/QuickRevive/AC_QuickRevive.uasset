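; Quick Revive perk component that speeds up its owner's regeneration and revive charge while active.
; On perk start, it modifies the owner's StatManagerComponent, shortening regeneration delay and tick, raising regeneration rate and adding flat revive charge rate.
; On removal, it calls the parent, then restores the three regeneration stats to base values through chained lookups, each gating the next.
; ReviveChargeRate is not reset here.
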(event `self.ReceiveBeginPlay`
  (`parent.ReceiveBeginPlay`))

(event `self.PerkStartEvent`
  (bind _returnvalue (`Actor.GetComponentByClass` (`self.GetOwner`) "/Script/ZombieFPS.StatManagerComponent"))
  (`StatManagerComponent.IncreaseStatMult` _returnvalue "RegenerationDelay" 0.75 false)
  (`StatManagerComponent.IncreaseStatMult` _returnvalue "RegenerationTick" 0.5 false)
  (`StatManagerComponent.IncreaseStatMult` _returnvalue "RegenerationRate" 2.0 false)
  (`StatManagerComponent.IncreaseStatFlat` _returnvalue "ReviveChargeRate" 10.0 false))

(event `self.PerkRemoveEvent`
  (bind _returnvalue (`Actor.GetComponentByClass` (`self.GetOwner`) "/Script/ZombieFPS.StatManagerComponent"))
  (bind (_outstat _returnvalue_2) (`StatManagerComponent.GetBaseStat` _returnvalue "RegenerationTick"))
  (bind (_outstat_2 _returnvalue_3) (`StatManagerComponent.GetBaseStat` _returnvalue "RegenerationRate"))
  (bind (_outstat_3 _returnvalue_4) (`StatManagerComponent.GetBaseStat` _returnvalue "RegenerationDelay"))
  (`parent.PerkRemoveEvent`)
  (if _returnvalue_4
    (`StatManagerComponent.ResetStatToPreviousValue` _returnvalue "RegenerationDelay" _outstat_3)
    (if _returnvalue_2
      (`StatManagerComponent.ResetStatToPreviousValue` _returnvalue "RegenerationTick" _outstat)
      (if _returnvalue_3
        (`StatManagerComponent.ResetStatToPreviousValue` _returnvalue "RegenerationRate" _outstat_2)))))