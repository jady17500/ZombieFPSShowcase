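; Double Tap perk component that boosts its owner's fire rate.
; On perk start it raises the FireRateMultiplier stat by 33 percent of the current value through the owner's StatManagerComponent and adds the perk icon to player 0's perk container UI.
; On perk removal it sets that stat back to its base value, if one is found, and leaves the icon untouched.
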(event `self.PerkStartEvent`
  (`StatManagerComponent.IncreaseStatPercentage` (`Actor.GetComponentByClass` (`self.GetOwner`) "/Script/ZombieFPS.StatManagerComponent") "FireRateMultiplier" 33.0 false)
  (bind _widget (message `/Game/FPS_Test/Code/Player/BPI_Player.GetPlayerUi` (`GameplayStatics.GetPlayerCharacter` 0)))
  (`/Game/FPS_Test/Code/UI/Components/WBP_PerkContainer.Add Perk Icon` (`/Game/FPS_Test/Code/UI/Pages/WBP_MainUI.WBP_PerkContainer` _widget) (`self.PerkIconBrush`)))

(event `self.PerkRemoveEvent`
  (bind _returnvalue (`Actor.GetComponentByClass` (`self.GetOwner`) "/Script/ZombieFPS.StatManagerComponent"))
  (bind (_outstat _returnvalue_2) (`StatManagerComponent.GetBaseStat` _returnvalue "FireRateMultiplier"))
  (if _returnvalue_2
    (`StatManagerComponent.ResetStatToPreviousValue` _returnvalue "FireRateMultiplier" _outstat)))