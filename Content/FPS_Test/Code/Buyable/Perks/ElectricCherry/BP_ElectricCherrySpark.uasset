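; Electric Cherry perk spark actor that follows its owner and halts nearby enemies while active.
; While IsActive, Tick snaps it to the owner, sphere-overlaps pawns of class BP_BaseEnemy within Radius and stops their AI controller movement, with optional debug drawing.
; IsActive replicates with a RepNotify that toggles visibility of the Niagara effect and reactivates it.
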(event `self.ReceiveBeginPlay`
  (`KismetSystemLibrary.PrintString` "Hello"))

(event `self.ReceiveTick`
  (params (DeltaSeconds :type "Float (single-precision)"))
  (bind _returnvalue (`self.GetOwner`))
  (bind _returnvalue_2 (`self.K2_GetActorLocation`))
  (bind _radius (`self.Radius`))
  (if (`self.IsActive`)
    (`self.K2_SetActorLocation` (`self.K2_GetActorLocation` _returnvalue))
    (bind _outactors (`KismetSystemLibrary.SphereOverlapActors` _returnvalue_2 _radius (`|MakeArray` "ObjectTypeQuery3" :!type "EObjectTypeQuery Enum") "/Game/FPS_Test/Code/Enemy/BP_BaseEnemy.BP_BaseEnemy_C" (`|MakeArray` _returnvalue)))
    (if (`self.DrawDebug`)
      (`KismetSystemLibrary.DrawDebugSphere` _returnvalue_2 _radius 12 (struct :`R` 1.0 :`G` 0.045253 :`A` 1.0) 0.1 4.0))
    (for _array_element _outactors
      (`Controller.StopMovement` (`AIBlueprintHelperLibrary.GetAIController` _array_element)))))

(fn `OnRep_IsActive`
  (`SceneComponent.SetHiddenInGame` (`self.Niagara`) (not (`self.IsActive`)) true)
  (`ActorComponent.Activate` (`self.Niagara`) true))

(fn `UserConstructionScript`)