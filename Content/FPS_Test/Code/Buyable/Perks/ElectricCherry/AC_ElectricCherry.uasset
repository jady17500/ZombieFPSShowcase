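; Perk component for Electric Cherry that gives the owning FPS player an electric spark effect tied to reloading.
; On perk start it binds to the player's reload begin and end events, and on removal it unbinds them and destroys the spark actor.
; A single BP_ElectricCherrySpark actor is spawned lazily on first activation, then reused by toggling its IsActive flag.
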(event `ActivateSparks`
  (bind _sparks (`self.Sparks`))
  (if (`KismetSystemLibrary.IsValid` _sparks)
    (set `/Game/FPS_Test/Code/Buyable/Perks/ElectricCherry/BP_ElectricCherrySpark.IsActive` true _sparks)
    (else
      (bind _returnvalue (`|SpawnActorFromClass` "/Game/FPS_Test/Code/Buyable/Perks/ElectricCherry/BP_ElectricCherrySpark.BP_ElectricCherrySpark_C" (`KismetMathLibrary.MakeTransform` (0.0 0.0 0.0)) "Undefined" "MultiplyWithRoot" (`self.GetOwner`) 100.0 null))
      (bind _output_get (set `self.Sparks` _returnvalue))
      (set `/Game/FPS_Test/Code/Buyable/Perks/ElectricCherry/BP_ElectricCherrySpark.IsActive` true _output_get))))

(event `DisableSparks`
  (bind _sparks (`self.Sparks`))
  (if (`KismetSystemLibrary.IsValid` _sparks)
    (set `/Game/FPS_Test/Code/Buyable/Perks/ElectricCherry/BP_ElectricCherrySpark.IsActive` false _sparks)))

(event `self.PerkRemoveEvent`
  (`parent.PerkRemoveEvent`)
  (bind _asbp_fpsplayer (cast `/Game/FPS_Test/Code/Player/BP_FPSPlayer` (`self.GetOwner`)))
  (remove `/Game/FPS_Test/Code/Player/BP_FPSPlayer.OnReloadBegin` _asbp_fpsplayer (`|CreateDelegate` :!event `ActivateSparks`))
  (remove `/Game/FPS_Test/Code/Player/BP_FPSPlayer.OnReloadEnd` _asbp_fpsplayer (`|CreateDelegate` :!event `DisableSparks`))
  (`Actor.K2_DestroyActor` (`self.Sparks`)))

(event `self.PerkStartEvent`
  (bind _asbp_fpsplayer (cast `/Game/FPS_Test/Code/Player/BP_FPSPlayer` (`self.GetOwner`)))
  (add `/Game/FPS_Test/Code/Player/BP_FPSPlayer.OnReloadBegin` _asbp_fpsplayer (`|CreateDelegate` :!event `ActivateSparks`))
  (add `/Game/FPS_Test/Code/Player/BP_FPSPlayer.OnReloadEnd` _asbp_fpsplayer (`|CreateDelegate` :!event `DisableSparks`)))