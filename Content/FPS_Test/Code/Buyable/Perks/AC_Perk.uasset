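; AC_Perk is an actor component for a buyable perk that manages the perk's icon in its owner's UI.
; On BeginPlay it gets the player UI message widget from its owner and adds PerkIconBrush to that widget's perk container.
; PerkRemoveEvent fetches the same widget and removes that icon from the container.
; The graph contains only this icon handling, with no gameplay effect.
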(event `self.ReceiveBeginPlay`
  (bind _widget (message `/Game/FPS_Test/Code/Player/BPI_Player.GetPlayerUi` (`self.GetOwner`)))
  (`/Game/FPS_Test/Code/UI/Components/WBP_PerkContainer.Add Perk Icon` (`/Game/FPS_Test/Code/UI/Pages/WBP_MainUI.WBP_PerkContainer` _widget) (`self.PerkIconBrush`)))

(event `self.PerkRemoveEvent`
  (bind _widget (message `/Game/FPS_Test/Code/Player/BPI_Player.GetPlayerUi` (`self.GetOwner`)))
  (`/Game/FPS_Test/Code/UI/Components/WBP_PerkContainer.RemovePerkIcon` (`/Game/FPS_Test/Code/UI/Pages/WBP_MainUI.WBP_PerkContainer` _widget) (`self.PerkIconBrush`)))