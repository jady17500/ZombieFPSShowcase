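; BP_PerkMachine is an interactable machine that sells a perk for in-game currency.
; On interact, it passes the interactor's currency component to its buyable component, unless the interactor already has the configured perk component.
; A completed purchase adds the perk component class to player 0's character rather than the interactor, and prints a debug string.
; The interaction prompt shows perk name, price, currency and description.
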(event `self.Interact`
  (params (Interactor :type "Actor Object Reference"))
  (`/Engine/EditorBlueprintResources/StandardMacros.IsValid` (`self.GetComponentByClass` Interactor (`self.PerkClass`))
    (:`Is Not Valid`
      (`BuyableComponent.Buy` (`self.AC_Buyable`) (`self.GetComponentByClass` Interactor "/Script/ZombieFPS.CurrencyComponent")))))

(event `self.AC_Buyable.OnBuyComplete`
  (`|AddComponentByClass` (`GameplayStatics.GetPlayerCharacter` 0) (`self.PerkClass`))
  (`KismetSystemLibrary.PrintString` "PerkBought"))

(fn `GetInteractText`
  (returns (OutText :type Text) (OutDescription :type Text) (ReturnValue :type Boolean))
  (bind _ac_buyable (`self.AC_Buyable`))
  (return (`|FormatText` "buy {NAME} for {PRICE} {CURRENCY_NAME}" (`self.PerkName`) (`BuyableComponent.Price` _ac_buyable) (`BuyableComponent.RequiredCurrencyName` _ac_buyable)) (`|FormatText` "[{DESCRIPTION}]" (`self.Description`)) true))

(fn `UserConstructionScript`)