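; Mule Kick perk component that gives its owner one extra weapon inventory slot while the perk is active.
; On perk start it adds a flat increase to the WeaponInventorySize stat through the owner's StatManagerComponent.
; On removal it runs the parent logic, then resets that stat to its base value rather than subtracting the bonus.
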(event `self.PerkStartEvent`
  (`StatManagerComponent.IncreaseStatFlat` (`Actor.GetComponentByClass` (`self.GetOwner`) "/Script/ZombieFPS.StatManagerComponent") "WeaponInventorySize" 1.0 false))

(event `self.PerkRemoveEvent`
  (bind _returnvalue (`Actor.GetComponentByClass` (`self.GetOwner`) "/Script/ZombieFPS.StatManagerComponent"))
  (`parent.PerkRemoveEvent`)
  (`StatManagerComponent.ResetStatToPreviousValue` _returnvalue "WeaponInventorySize" (`StatManagerComponent.GetBaseStat` _returnvalue "WeaponInventorySize")))