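; Pack-a-Punch interactable that sells the player an upgraded version of their active weapon.
; Interact looks up the active weapon's class in the "WeaponUpgrades" row map of UpgradesTable, then charges the interactor's CurrencyComponent through AC_Buyable.
; When the purchase completes, player 0, rather than the stored interactor, receives the upgrade class in place of their current weapon.
; The prompt shows the buyable's price and currency.
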(event `self.Interact`
  (params (Interactor :type "Actor Object Reference"))
  (bind _weapon_actor (message `/Game/FPS_Test/Code/Player/BPI_Player.GetActiveWeapon` Interactor))
  (bind _returnvalue (`|GetDataTableRow` (`self.UpgradesTable`) "WeaponUpgrades")
    (:`then`
      (bind (_value _returnvalue_2) (`BlueprintMapLibrary.Map_Find` (`.WeaponUpgrade_4_A455FB40439A18CF34ED17B84D5EE357` (break `/Game/FPS_Test/Code/Weapon/F_WeaponUpgrade` _returnvalue)) (castclass `/Game/FPS_Test/Code/Weapon/BP_LPAMG_WEP` (`GameplayStatics.GetObjectClass` _weapon_actor) :!pure true)))
      (if _returnvalue_2
        (set `self.FoundUpgrade` _value)
        (`BuyableComponent.Buy` (`self.AC_Buyable`) (`self.GetComponentByClass` Interactor "/Script/ZombieFPS.CurrencyComponent"))
        (else
          (`KismetSystemLibrary.PrintString` "UPGRADE NOT FOUND"))))
    (:`RowNotFound`
      (`KismetSystemLibrary.PrintString` "ROW NOT FOUND"))))

(event `self.AC_Buyable.OnBuyComplete`
  (message `/Game/FPS_Test/Code/Player/BPI_Player.AddWeaponToInventory` (`GameplayStatics.GetPlayerCharacter` 0) (`self.FoundUpgrade`) true))

(fn `GetInteractText`
  (returns (OutText :type Text) (OutDescription :type Text) (ReturnValue :type Boolean))
  (bind _ac_buyable (`self.AC_Buyable`))
  (return (`|FormatText` "Pack A Punch ({PRICE} {CURRENCY})" (`BuyableComponent.Price` _ac_buyable) (`BuyableComponent.RequiredCurrencyName` _ac_buyable)) "" true))

(fn `UserConstructionScript`)