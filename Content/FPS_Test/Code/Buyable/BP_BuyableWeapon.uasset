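; Buyable weapon pickup that shows a display model through a child actor and sells the weapon when interacted with.
; Interact passes the interactor's CurrencyComponent to AC_Buyable, whose OnBuyComplete adds WeaponClass to player 0's inventory without removing the current weapon, regardless of who interacted.
; The construction script sets the display from ShowCaseClass, and the prompt combines weapon name, price and currency.
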(event `self.ReceiveBeginPlay`
  (`parent.ReceiveBeginPlay`)
  (set `self.InteractText` (`self.InteractText`)))

(event `self.AC_Buyable.OnBuyComplete`
  (message `/Game/FPS_Test/Code/Player/BPI_Player.AddWeaponToInventory` (`GameplayStatics.GetPlayerCharacter` 0) (`self.WeaponClass`) false))

(event `self.Interact`
  (params (Interactor :type "Actor Object Reference"))
  (`BuyableComponent.Buy` (`self.AC_Buyable`) (`self.GetComponentByClass` Interactor "/Script/ZombieFPS.CurrencyComponent")))

(fn `GetInteractText`
  (returns (OutText :type Text) (OutDescription :type Text) (ReturnValue :type Boolean))
  (bind _ac_buyable (`self.AC_Buyable`))
  (return (`|FormatText` "buy {NAME}:{PRICE} {CURRENCY}" (`self.WeaponName`) (`BuyableComponent.Price` _ac_buyable) (`BuyableComponent.RequiredCurrencyName` _ac_buyable)) "" true))

(fn `UserConstructionScript`
  (`parent.UserConstructionScript`)
  (`ChildActorComponent.SetChildActorClass` (`self.ChildActor`) (`self.ShowCaseClass`)))