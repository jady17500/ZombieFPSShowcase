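; A buyable door that the player pays currency to open through an interact prompt showing price and currency.
; Interact passes the interactor's CurrencyComponent to AC_Buyable's Buy.
; When the buy limit is reached, a timeline lerps the door mesh from its relative location by a set offset to slide it open.
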(event `self.Interact`
  (params (Interactor :type "Actor Object Reference"))
  (`BuyableComponent.Buy` (`self.AC_Buyable`) (`self.GetComponentByClass` Interactor "/Script/ZombieFPS.CurrencyComponent")))

(event `self.AC_Buyable.OnBuyLimitReached`
  (`self.OpenDoor`))

(event `OpenDoor`
  (bind _relativelocation (`SceneComponent.RelativeLocation` (`self.DoorMesh`)))
  (set `self.StartPosition` _relativelocation)
  (set `self.EndPosition` (+ _relativelocation (`self.Offset`)))
  (bind (_direction _doorposition) (`Timeline|Timeline` :!via `PlayFromStart`)
    (:`Update`
      (`SceneComponent.K2_SetRelativeLocation` (`self.DoorMesh`) (`KismetMathLibrary.VLerp` (`self.StartPosition`) (`self.EndPosition`) _doorposition) false false))))

(fn `GetInteractText`
  (returns (OutText :type Text) (OutDescription :type Text) (ReturnValue :type Boolean))
  (bind _ac_buyable (`self.AC_Buyable`))
  (return (`|FormatText` "open door {PRICE} {CURRENCy}" (`BuyableComponent.Price` _ac_buyable) (`BuyableComponent.RequiredCurrencyName` _ac_buyable)) "" true))

(fn `UserConstructionScript`)