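; BP_ScaledEnemy is an enemy Blueprint that hands out drops and currency rewards in response to its AC_EnemyHealth events.
; On death, the authority asks the game mode's GameManagerComponent to spawn a drop, and a valid killer's CurrencyComponent gains currency by damage type.
; The actor is destroyed after a delay, except when a valid killer lacks that component.
; Non-lethal hits grant the attacker a small fixed reward.
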(event `self.ReceiveBeginPlay`
  (`parent.ReceiveBeginPlay`))

(event `self.AC_EnemyHealth.OnDeath`
  (params (Killer :type "Actor Object Reference") (DamageType :type "EDamageType Enum" :default "HEADSHOT"))
  (bind _returnvalue (`self.GetComponentByClass` Killer "/Script/ZombieFPS.CurrencyComponent"))
  ;[0.06678 0 0.15] Ideally I would do this in the game manager but I didn't have time to adapt the structure
  (`/Engine/EditorBlueprintResources/ActorMacros.Switch Has Authority`
    (:`Authority`
      (`GameManagerComponent.SpawnDrop` (`self.GetComponentByClass` (`GameplayStatics.GetGameMode`) "/Script/ZombieFPS.GameManagerComponent") (`self.GetTransform`)))
    (:`Remote`
      _))
  (`/Engine/EditorBlueprintResources/StandardMacros.IsValid` Killer
    (:`Is Valid`
      (`/Engine/EditorBlueprintResources/StandardMacros.IsValid` _returnvalue
        (:`Is Valid`
          (`CurrencyComponent.GainCurrency` _returnvalue (select `EDamageType` DamageType :`HEADSHOT` 100 :`BODYSHOT` 60 :`MELEE` 130 :`EXPLOSIVE` 50)))))
    (:`Is Not Valid`
      _))
  (`KismetSystemLibrary.Delay` 5.0)
  (`self.K2_DestroyActor`))

(event `self.AC_EnemyHealth.OnDamageTaken`
  (params (Attacker :type "Actor Object Reference") (DamageType :type "EDamageType Enum" :default "HEADSHOT"))
  (bind _returnvalue (`self.GetComponentByClass` Attacker "/Script/ZombieFPS.CurrencyComponent"))
  (if (> (`HealthComponent.CurrentHealth` (`self.AC_EnemyHealth`)) 0)
    (`/Engine/EditorBlueprintResources/StandardMacros.IsValid` _returnvalue
      (:`Is Valid`
        (`CurrencyComponent.GainCurrency` _returnvalue 10)))))

(fn `UserConstructionScript`
  (`parent.UserConstructionScript`))