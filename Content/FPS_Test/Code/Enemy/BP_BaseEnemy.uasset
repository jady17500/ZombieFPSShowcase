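; BP_BaseEnemy is an enemy character Blueprint that tracks its movement state and handles its own death.
; Tick sets IsMoving and IsRunning by comparing velocity length against walk and run thresholds.
; When the AC_EnemyHealth component fires OnDeath, the mesh ragdolls through physics simulation, capsule collision turns off, and the AI controller's brain logic stops.
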(event `self.ReceiveBeginPlay`)

(event `self.ReceiveTick`
  (params (DeltaSeconds :type "Float (single-precision)"))
  (bind _returnvalue (`KismetMathLibrary.VSize` (`self.GetVelocity`)))
  (set `self.IsMoving` (>= _returnvalue 0.1))
  (set `self.IsRunning` (>= _returnvalue 350.0)))

(event `self.AC_EnemyHealth.OnDeath`
  (params (Killer :type "Actor Object Reference") (DamageType :type "EDamageType Enum" :default "HEADSHOT"))
  (`PrimitiveComponent.SetSimulatePhysics` (`self.Mesh`) true)
  (`PrimitiveComponent.SetCollisionEnabled` (`self.CapsuleComponent`) "NoCollision")
  (bind _asaicontroller (cast `AIController` (`self.GetController`)))
  (`BrainComponent.StopLogic` (`AIController.BrainComponent` _asaicontroller) ""))

(fn `UserConstructionScript`)