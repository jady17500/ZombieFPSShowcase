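; BP_Projectile is an explosive projectile that detonates when its collision overlaps any actor other than the player character.
; It spawns an explosion effect at the hit actor, then damages health components on pawns within a sphere around itself before destroying itself.
; PlayerHealth takes fixed damage, while other health components take the Damage variable with the player as attacker.
; Debug print and sphere remain, and a TODO marks the damage logic for moving to AC_ShootComponent.
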(event `self.Collision.OnComponentBeginOverlap`
  (params (OverlappedComponent :type "PrimitiveComponent Object Reference") (OtherActor :type "Actor Object Reference") (OtherComp :type "PrimitiveComponent Object Reference") (OtherBodyIndex :type Integer) (bFromSweep :type Boolean) (SweepResult :type "HitResult Structure (by ref)"))
  (bind _returnvalue (`self.K2_GetActorLocation`))
  (if (!= OtherActor (`GameplayStatics.GetPlayerCharacter` 0))
    (`KismetSystemLibrary.PrintString` (`KismetSystemLibrary.GetDisplayName` OtherActor))
    (`GameplayStatics.SpawnEmitterAtLocation` "/Game/Realistic_Starter_VFX_Pack_Vol2/Particles/Explosion/P_Explosion_Big_A.P_Explosion_Big_A" (`self.K2_GetActorLocation` OtherActor))
    (bind _outactors (`KismetSystemLibrary.SphereOverlapActors` _returnvalue 90.0 (`|MakeArray` "ObjectTypeQuery3" :!type "EObjectTypeQuery Enum")))
    ; TODO: Move this to AC_ShootComponent
    (for _array_element _outactors
      (bind _returnvalue_2 (`self.GetComponentByClass` _array_element "/Script/ZombieFPS.HealthComponent"))
      (`/Engine/EditorBlueprintResources/StandardMacros.IsValid` _returnvalue_2
        (:`Is Valid`
          (bind _asplayer_health (cast `PlayerHealth` _returnvalue_2)
            (:`then`
              (`HealthComponent.Damage` _asplayer_health 90 null "EXPLOSIVE"))
            (:`CastFailed`
              (`HealthComponent.Damage` _returnvalue_2 (`self.Damage`) (`GameplayStatics.GetPlayerCharacter` 0) "EXPLOSIVE"))))))
    (`KismetSystemLibrary.DrawDebugSphere` _returnvalue 90.0 12 (struct :`G` 0.080975 :`B` 1.0 :`A` 1.0) 2.0 2.0)
    (`self.K2_DestroyActor`)))

(fn `UserConstructionScript`)