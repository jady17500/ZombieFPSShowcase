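; AC_ZombieBlood is a timed component for the Zombie Blood drop that temporarily changes how enemies prioritize its owner as a target.
; On BeginPlay it sets the owner's AC_EnemyTarget priority to 0.
; Tick counts Lifetime down, then sets the priority to 1 and destroys the component, without saving the earlier priority.
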(event `self.ReceiveBeginPlay`
  (`EnemyTargetComponent.ChangePriority` (`Actor.GetComponentByClass` (`self.GetOwner`) "/Game/FPS_Test/Code/Enemy/AC_EnemyTarget.AC_EnemyTarget_C") 0))

(event `self.ReceiveTick`
  (params (DeltaSeconds :type "Float (single-precision)"))
  (bind _output_get (set `self.Lifetime` (- (`self.Lifetime`) DeltaSeconds)))
  (if (<= _output_get 0.0)
    (`EnemyTargetComponent.ChangePriority` (`Actor.GetComponentByClass` (`self.GetOwner`) "/Game/FPS_Test/Code/Enemy/AC_EnemyTarget.AC_EnemyTarget_C") 1)
    (`self.K2_DestroyComponent`)))