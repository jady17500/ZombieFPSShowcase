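; BP_BaseDrop is the base pickup for timed bonus drops, destroying itself once its Lifetime expires.
; When BP_FPSPlayer overlaps its sphere, it adds a WBP_BonusCard with the bonus name and duration to the player's UI message widget.
; It then calls ActivateBonus on that player and destroys itself.
; ActivateBonus is empty here, serving as the hook for child drops to define their effect.
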(event `self.ReceiveBeginPlay`
  (`KismetSystemLibrary.Delay` (`self.Lifetime`))
  (`self.K2_DestroyActor`))

(event `self.Sphere.OnComponentBeginOverlap`
  (params (OverlappedComponent :type "PrimitiveComponent Object Reference") (OtherActor :type "Actor Object Reference") (OtherComp :type "PrimitiveComponent Object Reference") (OtherBodyIndex :type Integer) (bFromSweep :type Boolean) (SweepResult :type "HitResult Structure (by ref)"))
  (bind _asbp_fpsplayer (cast `/Game/FPS_Test/Code/Player/BP_FPSPlayer` OtherActor))
  (bind _returnvalue (`|CreateWidget` "/Game/FPS_Test/Code/UI/Components/WBP_BonusCard.WBP_BonusCard_C" null (`self.BonusName`) (`self.Duration`)))
  (bind _widget (message `/Game/FPS_Test/Code/Player/BPI_Player.GetPlayerUi` _asbp_fpsplayer))
  (`/Game/FPS_Test/Code/UI/Pages/WBP_MainUI.AddBonusCard` _widget _returnvalue)
  (`self.ActivateBonus` _asbp_fpsplayer)
  (`self.K2_DestroyActor`))

(fn `ActivateBonus`
  (params (PlayerActor :type "Actor Object Reference")))

(fn `UserConstructionScript`)