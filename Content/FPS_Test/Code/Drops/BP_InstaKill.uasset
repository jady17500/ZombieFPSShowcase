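; BP_InstaKill is an insta-kill bonus drop that temporarily gives the player an enormous damage multiplier.
; It overrides ActivateBonus, calls the parent, then adds a huge flat increase to the DamageMultiplier stat through the player's StatManagerComponent for the Duration variable's length.
; The boost applies only when the current multiplier is at or below one, so it does not stack on an already raised multiplier.
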(fn `ActivateBonus`
  (params (PlayerActor :type "Actor Object Reference"))
  (bind _returnvalue (`self.GetComponentByClass` PlayerActor "/Script/ZombieFPS.StatManagerComponent"))
  (`parent.ActivateBonus` PlayerActor)
  (if (<= (`StatManagerComponent.GetStat` _returnvalue "DamageMultiplier") 1.0)
    (`StatManagerComponent.IncreaseStatFlatForDuration` _returnvalue "DamageMultiplier" 9999999.0 true (`self.Duration`))))

(fn `UserConstructionScript`
  (`parent.UserConstructionScript`))