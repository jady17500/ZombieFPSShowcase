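; BP_Nuke is a bonus drop that wipes out enemies and rewards the activating player.
; It overrides ActivateBonus, runs the parent logic, then finds every BP_BaseEnemy actor and triggers Death on its HealthComponent as a body shot.
; It then grants a flat currency payout through the player's CurrencyComponent, independent of how many enemies die.
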(fn `ActivateBonus`
  (params (PlayerActor :type "Actor Object Reference"))
  (`parent.ActivateBonus` PlayerActor)
  (bind _outactors (`GameplayStatics.GetAllActorsOfClass` "/Game/FPS_Test/Code/Enemy/BP_BaseEnemy.BP_BaseEnemy_C"))
  (for _array_element _outactors
    (`HealthComponent.Death` (`self.GetComponentByClass` _array_element "/Script/ZombieFPS.HealthComponent") null "BODYSHOT"))
  (`CurrencyComponent.GainCurrency` (`self.GetComponentByClass` PlayerActor "/Script/ZombieFPS.CurrencyComponent") 400))

(fn `UserConstructionScript`
  (`parent.UserConstructionScript`))