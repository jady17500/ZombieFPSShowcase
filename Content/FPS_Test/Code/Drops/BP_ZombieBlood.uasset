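; Zombie Blood drop, a bonus that gives the player an AC_ZombieBlood component when activated.
; ActivateBonus calls the parent, then checks the player for that component, extending its Lifetime by Duration if present and adding a new one otherwise.
; Repeat activations stack time on a single component, which holds the effect itself; the event graph is empty apart from disabled stubs.
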(fn `ActivateBonus`
  (params (PlayerActor :type "Actor Object Reference"))
  (bind _returnvalue (`self.GetComponentByClass` PlayerActor "/Game/FPS_Test/Code/Drops/AC_ZombieBlood.AC_ZombieBlood_C"))
  (`parent.ActivateBonus` PlayerActor)
  (`/Engine/EditorBlueprintResources/StandardMacros.IsValid` _returnvalue
    (:`Is Valid`
      (set `/Game/FPS_Test/Code/Drops/AC_ZombieBlood.Lifetime` (+ (`/Game/FPS_Test/Code/Drops/AC_ZombieBlood.Lifetime` _returnvalue) (`self.Duration`)) _returnvalue))
    (:`Is Not Valid`
      (`|AddComponentByClass` PlayerActor "/Game/FPS_Test/Code/Drops/AC_ZombieBlood.AC_ZombieBlood_C"))))

(fn `UserConstructionScript`
  (`parent.UserConstructionScript`))