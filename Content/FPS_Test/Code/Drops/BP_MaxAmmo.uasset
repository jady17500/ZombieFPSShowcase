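; BP_MaxAmmo is a drop bonus that refills ammo on every weapon the activating player carries.
; It overrides the parent's ActivateBonus, calls the parent, then calls RefillAmmo on the ShootComponent of each valid weapon in the player's inventory.
; It then reads the active weapon's ammo and updates the player UI's ammo text, using message calls to reach player, weapon and UI.
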(fn `ActivateBonus`
  (params (PlayerActor :type "Actor Object Reference"))
  (`parent.ActivateBonus` PlayerActor)
  (bind _inventory (message `/Game/FPS_Test/Code/Player/BPI_Player.GetWeaponInventory` PlayerActor))
  (for _array_element _inventory
    (`/Engine/EditorBlueprintResources/StandardMacros.IsValid` _array_element
      (:`Is Valid`
        (`ShootComponent.RefillAmmo` (`self.GetComponentByClass` _array_element "/Script/ZombieFPS.ShootComponent")))))
  (bind _weapon_actor (message `/Game/FPS_Test/Code/Player/BPI_Player.GetActiveWeapon` PlayerActor))
  (`/Engine/EditorBlueprintResources/StandardMacros.IsValid` _weapon_actor
    (:`Is Valid`
      (bind _widget (message `/Game/FPS_Test/Code/Player/BPI_Player.GetPlayerUi` PlayerActor))
      (bind (_reserveammo _currentammo) (message `/Game/LowPolyAnimatedModernGuns/Demo/Core/Weapons/BPI_LPAMG_WEP.GetAmmo` _weapon_actor))
      (`/Game/FPS_Test/Code/UI/Pages/WBP_MainUI.Set Ammo Text` _widget _currentammo _reserveammo))))

(fn `UserConstructionScript`
  (`parent.UserConstructionScript`))