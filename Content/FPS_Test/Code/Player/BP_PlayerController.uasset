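; Player controller for the FPS test game that sets up input and handles the pause menu.
; On BeginPlay it adds the IMC_FPS Enhanced Input mapping context and switches to game-only input.
; IA_Pause pauses the game and pushes a new pause menu onto the GameMode's AC_WidgetStack.
; While paused, it pops the top widget, unpausing only when that widget is the pause menu itself.
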(event `self.ReceiveBeginPlay`
  (`EnhancedInputSubsystemInterface.AddMappingContext` (subsystem `EnhancedInputLocalPlayerSubsystem`) "/Game/FPS_Test/Data/Input/IMC_FPS.IMC_FPS" 0 (struct))
  (`WidgetBlueprintLibrary.SetInputMode_GameOnly` self))

(event `EnhancedInput|/Game/FPS_Test/Data/Input/IA_Pause`
  (params (ActionValue :type Boolean) (ElapsedSeconds :type "Float (double-precision)") (TriggeredSeconds :type "Float (double-precision)") (InputAction :type "InputAction Object Reference" :default "/Game/FPS_Test/Data/Input/IA_Pause.IA_Pause"))
  (bind _returnvalue (`self.GetComponentByClass` (`GameplayStatics.GetGameMode`) "/Game/FPS_Test/Code/Core/AC_WidgetStack.AC_WidgetStack_C"))
  (:`Triggered`
    (if (`GameplayStatics.IsGamePaused`)
      (if (== (`GameplayStatics.GetObjectClass` (`ActionStackComponent.CurrentAction` _returnvalue)) (`self.PauseMenuClass`))
        (`ActionStackComponent.PopAction` _returnvalue)
        (`/Game/FPS_Test/Code/Utility/BPFL_Utility.UnPauseGame` self)
        (else
          (`ActionStackComponent.PopAction` _returnvalue)))
      (else
        (`/Game/FPS_Test/Code/Utility/BPFL_Utility.PauseGame` self)
        (bind _returnvalue_2 (`|CreateWidget` (`self.PauseMenuClass`)))
        (`ActionStackComponent.PushAction` _returnvalue _returnvalue_2)))))

(fn `UserConstructionScript`)