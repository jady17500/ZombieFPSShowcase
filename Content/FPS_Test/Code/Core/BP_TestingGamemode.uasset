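; BP_TestingGamemode is a test game mode for the FPS that sets up the player's main UI and handles player death.
; On BeginPlay it pushes WBP_MainUI through ACWidgetStack, hands it to BP_FPSPlayer and binds to the PlayerHealth component's death event.
; On death it pushes WBP_GameOver with a round number of zero, shows the cursor and switches input to UI only.
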(event `self.ReceiveBeginPlay`
  (bind _returnvalue (`|CreateWidget` "/Game/FPS_Test/Code/UI/Pages/WBP_MainUI.WBP_MainUI_C"))
  (`ActionStackComponent.PushAction` (`self.AC_WidgetStack`) _returnvalue)
  (bind _asbp_fpsplayer (cast `/Game/FPS_Test/Code/Player/BP_FPSPlayer` (`GameplayStatics.GetPlayerCharacter` 0)))
  (set `/Game/FPS_Test/Code/Player/BP_FPSPlayer.MainUI` _returnvalue _asbp_fpsplayer)
  (add `HealthComponent.OnDeath` (`self.GetComponentByClass` (`GameplayStatics.GetPlayerCharacter` 0) "/Script/ZombieFPS.PlayerHealth") (`|CreateDelegate` :!event `OnPlayerDeath`)))

(event `OnPlayerDeath`
  (params (Killer :type "Actor Object Reference") (DamageType :type "EDamageType Enum" :default "HEADSHOT"))
  (bind _returnvalue (`GameplayStatics.GetPlayerController` 0))
  (bind _returnvalue_2 (`|CreateWidget` "/Game/FPS_Test/Code/UI/Pages/WBP_GameOver.WBP_GameOver_C"))
  (`ActionStackComponent.PushAction` (`self.AC_WidgetStack`) _returnvalue_2)
  (set `PlayerController.bShowMouseCursor` true _returnvalue)
  (`WidgetBlueprintLibrary.SetInputMode_UIOnlyEx` _returnvalue _returnvalue_2))

(fn `UserConstructionScript`)