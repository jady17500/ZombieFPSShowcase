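; Widget stack component that keeps a single UI widget visible among the entries of an action stack.
; On BeginPlay it binds DisplayFirstWidget to both the action-added and action-removed events.
; That handler loops through ActionStack, casts entries to UserWidget, makes the one matching the event's action visible and collapses the others.
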(event `self.ReceiveBeginPlay`
  (add `self.OnActionAdded` (delegate `DisplayFirstWidget`))
  (add `self.OnActionRemoved` (delegate `DisplayFirstWidget`)))

(event `DisplayFirstWidget` :!signature `self.OnActionAdded`
  (params (NewAction :type "Object Object Reference"))
  (for _array_element (`self.ActionStack`)
    (if (== _array_element NewAction)
      (bind _asuser_widget (cast `UserWidget` _array_element))
      (`Widget.SetVisibility` _asuser_widget "Visible")
      (else
        (bind _asuser_widget_2 (cast `UserWidget` _array_element))
        (`Widget.SetVisibility` _asuser_widget_2 "Collapsed")))))