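; AG14W weapon Blueprint that extends its parent with a swappable forestock and a separate front ironsight.
; Overrides add both meshes to skinning and attachment randomization, parent grip, muzzle and laser sockets to the forestock, and register it as a socket.
; Forestock choice drives attachment icons, while scope choice selects ironsight meshes and folded icon variants.
; Tick prints the Spread stat as debug output.
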(event `self.ReceiveBeginPlay`
  (`parent.ReceiveBeginPlay`))

(event `self.ReceiveTick`
  (params (DeltaSeconds :type "Float (single-precision)"))
  (`KismetSystemLibrary.PrintString` (`KismetStringLibrary.Conv_DoubleToString` (`StatManagerComponent.GetStat` (`self.AC_WeaponStatManager`) "Spread")) true true (struct :`G` 0.66 :`B` 1.0 :`A` 1.0) 2.0 "aaaa"))

(fn `Apply Selected Skin`
  (bind _skin_equipped (`self.Skin Equipped`))
  (`parent.Apply Selected Skin`)
  (`/Game/LowPolyAnimatedModernGuns/Demo/Core/Skins/BP_LPAMG_Skin.Apply To` _skin_equipped (`self.Mesh Forestock`) "Forestock")
  (`/Game/LowPolyAnimatedModernGuns/Demo/Core/Skins/BP_LPAMG_Skin.Apply To` _skin_equipped (`self.Mesh Ironsight Front`) "Ironsights"))

(fn `FoldIronsight`
  (`parent.FoldIronsight`)
  (`StaticMeshComponent.SetStaticMesh` (`self.Mesh Ironsight Front`) (`self.FoldedIronSightFront`)))

(fn `Get Socket Grip Parent`
  (returns (Parent :type "SceneComponent Object Reference") (`Socket Name` :type Name))
  (return (`self.Mesh Forestock`) (`.Socket Name` (`parent.Get Socket Grip Parent`))))

(fn `Get Socket Laser Parent`
  (returns (Parent :type "SceneComponent Object Reference") (`Socket Name` :type Name))
  (return (`self.Mesh Forestock`) (`.Socket Name` (`parent.Get Socket Laser Parent`))))

(fn `Get Socket Muzzle Parent`
  (returns (Parent :type "SceneComponent Object Reference") (`Socket Name` :type Name))
  (return (`self.Mesh Forestock`) (`.Socket Name` (`parent.Get Socket Muzzle Parent`))))

(fn `InitSockets`
  (`parent.InitSockets`)
  (`BlueprintMapLibrary.Map_Add` (`self.Sockets`) "Forestock" (`self.Mesh Forestock`)))

(fn `LPAMG - Get Texture Icon Forestock`
  (returns (ReturnValue :type "Texture2D Object Reference"))
  (return (`|GetArrayItem` (`self.Array Texture Icon Forestocks`) (`KismetArrayLibrary.Array_Find` (`self.Array Static Mesh Forestocks`) (`StaticMeshComponent.StaticMesh` (`self.Mesh Forestock`))))))

(fn `LPAMG - Get Texture Icon Ironsights Back`
  (returns (ReturnValue :type "Texture2D Object Reference"))
  (return (select `int` (`KismetArrayLibrary.Array_Find` (`self.Array Static Mesh Scopes`) (`StaticMeshComponent.StaticMesh` (`self.Mesh Scope`))) :`0` (`|GetArrayItem` (`self.Array Texture Icon Ironsights Back`) (`KismetArrayLibrary.Array_Find` (`self.Array Static Mesh Forestocks`) (`StaticMeshComponent.StaticMesh` (`self.Mesh Forestock`)))) :`1` (`|GetArrayItem` (`self.Array Texture Icon Ironsights Back Folded`) (`KismetArrayLibrary.Array_Find` (`self.Array Static Mesh Forestocks`) (`StaticMeshComponent.StaticMesh` (`self.Mesh Forestock`)))))))

(fn `LPAMG - Get Texture Icon Ironsights Front`
  (returns (ReturnValue :type "Texture2D Object Reference"))
  (return (select `int` (`KismetArrayLibrary.Array_Find` (`self.Array Static Mesh Scopes`) (`StaticMeshComponent.StaticMesh` (`self.Mesh Scope`))) :`0` (`|GetArrayItem` (`self.Array Texture Icon Ironsights Front`) (`KismetArrayLibrary.Array_Find` (`self.Array Static Mesh Forestocks`) (`StaticMeshComponent.StaticMesh` (`self.Mesh Forestock`)))) :`1` (`|GetArrayItem` (`self.Array Texture Icon Ironsights Front Folded`) (`KismetArrayLibrary.Array_Find` (`self.Array Static Mesh Forestocks`) (`StaticMeshComponent.StaticMesh` (`self.Mesh Forestock`)))))))

(fn `LPAMG - Get Texture Icon Muzzle`
  (returns (ReturnValue :type "Texture2D Object Reference"))
  (return (select `bool` (== (`KismetArrayLibrary.Array_Find` (`self.Array Static Mesh Muzzles`) (`StaticMeshComponent.StaticMesh` (`self.Mesh Muzzle`))) 0) :`false` (select `bool` (`self.Are Attachments Visible Pure`) :`true` (`|GetArrayItem` (`self.Array Texture Icon Muzzles Extended`) (`KismetArrayLibrary.Array_Find` (`self.Array Static Mesh Forestocks`) (`StaticMeshComponent.StaticMesh` (`self.Mesh Forestock`))))))))

(fn `Randomize Attachment Meshes`
  (`parent.Randomize Attachment Meshes`)
  (`StaticMeshComponent.SetStaticMesh` (`self.Mesh Forestock`) (`KismetArrayLibrary.Array_Random` (`self.Array Static Mesh Forestocks`)) :!pinned true) ; Forestock
  (`StaticMeshComponent.SetStaticMesh` (`self.Mesh Ironsights`) (`|GetArrayItem` (`self.Array Static Mesh Ironsights Back`) (`KismetArrayLibrary.Array_Find` (`self.Array Static Mesh Scopes`) (`StaticMeshComponent.StaticMesh` (`self.Mesh Scope`))))) ; Ironsights. This node helps with adding\nthe folding setup.
  (`StaticMeshComponent.SetStaticMesh` (`self.Mesh Ironsight Front`) (`|GetArrayItem` (`self.Array Static Mesh Ironsights Front`) (`KismetArrayLibrary.Array_Find` (`self.Array Static Mesh Scopes`) (`StaticMeshComponent.StaticMesh` (`self.Mesh Scope`))))) ; Ironsights. This node helps with adding\nthe folding setup.
)

(fn `Randomize Skin`
  (`parent.Randomize Skin`)
  (`/Game/LowPolyAnimatedModernGuns/Demo/Core/Skins/BP_LPAMG_Skin.Apply To` (`self.Skin Equipped`) (`self.Mesh Forestock`) "Forestock") ; Forestock
  (`/Game/LowPolyAnimatedModernGuns/Demo/Core/Skins/BP_LPAMG_Skin.Apply To` (`self.Skin Equipped`) null "Barrel") ; Barrel
  (`/Game/LowPolyAnimatedModernGuns/Demo/Core/Skins/BP_LPAMG_Skin.Apply To` (`self.Skin Equipped`) (`self.Mesh Ironsight Front`) "Ironsights") ; Ironsights
)

(fn `UserConstructionScript`
  (`parent.UserConstructionScript`))